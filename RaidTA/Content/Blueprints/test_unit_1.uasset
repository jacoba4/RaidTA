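; Test unit actor that carries a HealthUI widget component and tracks its health as a percentage.
; On BeginPlay it casts the component's widget to HealthUI, hands it a reference to itself, then runs SetPercent through that reference.
; SetPercent divides Hp by MaxHp, capped at full, into HealthPercentage.
; The CallSetPercent event repeats that calculation on demand through the widget's unit reference.
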(event `self.CallSetPercent`
  (`self.SetPercent` (stale `self.ReceiveBeginPlay` _output_get)))

(event `self.ReceiveBeginPlay`
  (bind _ashealth_ui (cast `/Game/Blueprints/HealthUI` (`WidgetComponent.GetUserWidgetObject` (`self.HealthUI`))))
  (bind _output_get (set `/Game/Blueprints/HealthUI.Test_Unit` self _ashealth_ui))
  (`self.SetPercent` _output_get))

(fn `SetPercent`
  (set `self.HealthPercentage` (`KismetMathLibrary.FMin` (/ (`KismetMathLibrary.Conv_IntToDouble` (`self.hp`)) (`KismetMathLibrary.Conv_IntToDouble` (`self.max_hp`))) 1.0)))

(fn `UserConstructionScript`)